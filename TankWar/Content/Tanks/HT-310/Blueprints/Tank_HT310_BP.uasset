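; Player-controllable HT-310 tank pawn that can move, rotate, fly and fire.
; On BeginPlay it hands its four corner motors (front and back, left and right) to MovementComponent.
; Movement, rotation and fly axis inputs pass straight to that component, while the Fire press calls a Fire function not defined in this Blueprint.
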(event `self.ReceiveBeginPlay`
  (`MovementComponent_HT310.Initialise` (`self.MovementComponent`) (`self.Motor_BL`) (`self.Motor_BR`) (`self.Motor_FL`) (`self.Motor_FR`)))

(event `InputAxis|MoveForward`
  (params (AxisValue :type "Float (single-precision)"))
  (`MovementComponent_HT310.MoveForward` (`self.MovementComponent`) AxisValue))

(event `InputAction|Fire`
  (params (Key :type "Key Structure"))
  (:`Pressed`
    (`self.Fire`)))

(event `InputAxis|MoveRight`
  (params (AxisValue :type "Float (single-precision)"))
  (`MovementComponent_HT310.MoveRight` (`self.MovementComponent`) AxisValue))

(event `InputAxis|Rotation`
  (params (AxisValue :type "Float (single-precision)"))
  (`MovementComponent_HT310.Rotate` (`self.MovementComponent`) AxisValue))

(event `InputAxis|Fly`
  (params (AxisValue :type "Float (single-precision)"))
  (`MovementComponent_HT310.fly` (`self.MovementComponent`) AxisValue))

(fn `UserConstructionScript`)