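; HT310_BP is the HT-310 tank Blueprint, which routes player input to tank movement.
; On BeginPlay it initialises its MovementComponent with four corner motors: back-left, back-right, front-left and front-right.
; MoveForward and MoveRight axis inputs, labelled as locked-mode movement, pass straight to that component.
; The Rotation axis bypasses it, applying the raw axis value as local yaw to the Tank component.
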(event `self.ReceiveBeginPlay`
  (`MovementComponent_HT310.Initialise` (`self.MovementComponent`) (`self.Motor_BL`) (`self.Motor_BR`) (`self.Motor_FL`) (`self.Motor_FR`)))

(event `InputAxis|MoveForward`
  (params (AxisValue :type "Float (single-precision)"))
  ;[1 1 1] Locked mod Movement
  (`MovementComponent_HT310.MoveForward` (`self.MovementComponent`) AxisValue))

(event `InputAxis|MoveRight`
  (params (AxisValue :type "Float (single-precision)"))
  ;[1 1 1] Locked mod Movement
  (`MovementComponent_HT310.MoveRight` (`self.MovementComponent`) AxisValue))

(event `InputAxis|Rotation`
  (params (AxisValue :type "Float (single-precision)"))
  ;[1 1 1] Locked mod Movement
  (`SceneComponent.K2_AddLocalRotation` (`self.Tank`) (`KismetMathLibrary.MakeRotator` 0.0 0.0 AxisValue) false false))

(fn `UserConstructionScript`)